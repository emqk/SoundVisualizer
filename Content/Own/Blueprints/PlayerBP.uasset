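; PlayerBP is an orbiting viewpoint actor that circles and faces a RotateAroundBP actor found at BeginPlay.
; Each Tick moves it along local X by MoveSpeed, then, if the target is valid, advances a yaw angle by RotationSpeed.
; That angle places it at Distance and CameraHeight around the target, replacing the forward move, and a look-at rotation turns it toward the target.
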(event `self.ReceiveBeginPlay`
  (bind _returnvalue (`GameplayStatics.GetActorOfClass` "/Game/Own/Blueprints/RotateAroundBP.RotateAroundBP_C"))
  (set `self.RotateAround` _returnvalue))

(event `self.ReceiveTick`
  (params (DeltaSeconds :type "Float (single-precision)"))
  (`self.K2_AddActorLocalOffset` (`KismetMathLibrary.MakeVector` (* DeltaSeconds (`self.MoveSpeed`))))
  (`/Engine/EditorBlueprintResources/StandardMacros.IsValid` (`self.RotateAround`)
    (:`Is Valid`
      (`self.RotateAroundTarget` DeltaSeconds)
      (`self.LookAtTarget`))))

(fn `LookAtTarget`
  (`self.K2_SetActorRotation` (`KismetMathLibrary.FindLookAtRotation` (`self.K2_GetActorLocation`) (`self.K2_GetActorLocation` (`self.RotateAround`)))))

(fn `RotateAroundTarget`
  (params (DeltaTime :type "Float (double-precision)"))
  (bind _output_get (set `self.CurrRotation` (+ (* DeltaTime (`self.RotationSpeed`)) (`self.CurrRotation`))))
  (`self.K2_SetActorLocation` (+ (+ (`self.K2_GetActorLocation` (`self.RotateAround`)) (* (`KismetMathLibrary.GreaterGreater_VectorRotator` (`KismetMathLibrary.MakeVector` -1.0) (`KismetMathLibrary.MakeRotator` 0.0 0.0 _output_get)) (`self.Distance`))) (`KismetMathLibrary.MakeVector` 0.0 0.0 (`self.CameraHeight`))) true true))

(fn `UserConstructionScript`)