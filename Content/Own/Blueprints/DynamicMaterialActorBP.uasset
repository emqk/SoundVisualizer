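; Actor Blueprint that smoothly blends a static mesh's material through a "LerpAmount" scalar parameter.
; The construction script creates a dynamic material instance on the mesh's first slot.
; SetDynamicMaterialColorAmount stores the given amount as the target only if it reaches GangThreshold, otherwise zero.
; Tick interpolates the parameter toward that target at LerpSpeed.
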(event `self.ReceiveBeginPlay`)

(event `self.ReceiveTick`
  (params (DeltaSeconds :type "Float (single-precision)"))
  (bind _returnvalue (`MaterialInstanceDynamic.K2_GetScalarParameterValue` (`self.DynamicMat`) "LerpAmount"))
  (`MaterialInstanceDynamic.SetScalarParameterValue` (`self.DynamicMat`) "LerpAmount" (`KismetMathLibrary.FInterpTo` _returnvalue (`self.ColorAmount`) DeltaSeconds (`self.LerpSpeed`))))

(fn `SetDynamicMaterialColorAmount`
  (params (Amount01 :type "Float (double-precision)"))
  (if (>= Amount01 (`self.GangThreshold`))
    (set `self.ColorAmount` Amount01)
    (else
      (set `self.ColorAmount` 0.0))))

(fn `UserConstructionScript`
  (bind _returnvalue (`PrimitiveComponent.CreateDynamicMaterialInstance` (`self.StaticMesh`) 0 (`self.DyanmicMaterial`) "None"))
  (set `self.DynamicMat` _returnvalue))