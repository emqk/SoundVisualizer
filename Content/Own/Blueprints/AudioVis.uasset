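; Music visualizer actor that plays a track and drives visuals from baked audio analysis (Constant-Q, onsets) sampled at the playback position.
; Spectrum values scale a row of instanced mesh nodes, marking render state dirty once per refresh.
; Tick reads upcoming onsets to ease cube scale and point light intensity, spawning particles on strong hits.
; A spawned text actor shows Data Table lyrics timed by game time, not playback position.
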(event `self.ReceiveBeginPlay`
  (`self.SpawnNodes`)
  (`AudioComponent.SetSound` (`self.Audio`) (`self.AudioClip`))
  (add `AudioComponent.OnAudioPlaybackPercent` (`self.Audio`) (delegate `OnAudioPlaybackPercent_Event_0`))
  (`AudioComponent.Play` (`self.Audio`) 0.0)
  (bind _returnvalue (`|SpawnActorFromClass` (`self.TextToSpawn`) (`KismetMathLibrary.MakeTransform` (-1000.0 11500.0 200.0) (struct) (3.0 3.0 3.0)) "Undefined" "OverrideRootScale" null null))
  (set `self.SpawnedText` _returnvalue))

(event `OnAudioPlaybackPercent_Event_0`
  (params (PlayingSoundWave :type "SoundWave Object Reference") (PlaybackPercent :type "Float (double-precision)"))
  (bind _returnvalue (* PlaybackPercent (`self.Duration`)))
  (`KismetSystemLibrary.PrintString` (`KismetStringLibrary.Conv_DoubleToString` (`LoudnessNRT.GetNormalizedChannelLoudnessAtTime` (`self.LoudnessAnalizer`) _returnvalue 0)))
  (set `self.SpectrumValues` (`ConstantQNRT.GetNormalizedChannelConstantQAtTime` (`self.ConstantQ`) _returnvalue 0))
  (`self.RefreshNodes`))

(event `self.ReceiveTick`
  (params (DeltaSeconds :type "Float (single-precision)"))
  ;[1 1 1] Onset detection
  (bind _returnvalue (* (stale `OnAudioPlaybackPercent_Event_0` PlaybackPercent) (`self.Duration`)))
  (bind (_outonsettimestamps _outonsetstrengths) (`OnsetNRT.GetNormalizedChannelOnsetsBetweenTimes` (`self.Onset`) _returnvalue (+ _returnvalue 0.05) 0))
  (if (> (`KismetArrayLibrary.Array_Length` _outonsetstrengths) 0)
    (bind _output_get (set `self.CurrentOnset` (`|GetArrayItem` _outonsetstrengths)))
    (`KismetSystemLibrary.PrintString` (`KismetStringLibrary.Conv_DoubleToString` (`self.CurrentOnset`)) true true (struct :`R` 1.0 :`B` 0.83077 :`A` 1.0))
    (`self.SetOnsetCubeScale` _output_get DeltaSeconds)
    (`self.SetIntensityToLights` (`self.CurrentOnset`) DeltaSeconds)
    (if (>= (`self.CurrentOnset`) (`self.ToSpawnEmitterOnsetThreshold`))
      (`self.SpawnEmitter`)
      (`self.TickText` :!label _label))
    (else
      (set `self.CurrentOnset` 0.0)
      (`KismetSystemLibrary.PrintString` (`KismetStringLibrary.Conv_DoubleToString` (`self.CurrentOnset`)) true true (struct :`R` 1.0 :`B` 0.83077 :`A` 1.0))
      (goto _label))))

(fn `FindTargetText`
  (returns (Result :type Text))
  (locals (CurrentFinalText :type Text :default "NSLOCTEXT(\"\", \"EBC48B394512EE86AE714F9E56482A07\", \"[NO FOUND]\")"))
  (bind _lyricsdata (`self.LyricsData`))
  (bind _outrownames (`DataTableFunctionLibrary.GetDataTableRowNames` _lyricsdata))
  (for _array_element _outrownames
    (bind _returnvalue (`|GetDataTableRow` _lyricsdata _array_element)
      (:`then`
        (bind (_textstart _text) (break `/Game/Own/Blueprints/Text/MusicLyricsElement` _returnvalue))
        (if (>= (`KismetSystemLibrary.GetGameTimeInSeconds`) _textstart)
          (set `local.CurrentFinalText` _text)))
      (:`RowNotFound`
        (return (`local.CurrentFinalText`)))))
  (return (`local.CurrentFinalText`)))

(fn `RefreshNodes`
  (bind _instancedstaticmesh (`self.InstancedStaticMesh`))
  (bind _instancedstaticmesh_2 (`self.InstancedStaticMesh`))
  (bind _returnvalue (- (`KismetMathLibrary.Min` (`InstancedStaticMeshComponent.GetInstanceCount` _instancedstaticmesh_2) (`KismetArrayLibrary.Array_Length` (`self.SpectrumValues`))) 1))
  ;[1 1 1] Refresh every node
  (for _index (range (+ _returnvalue 1))
    (`InstancedStaticMeshComponent.UpdateInstanceTransform` (`self.InstancedStaticMesh`) _index (`KismetMathLibrary.MakeTransform` (.location (`InstancedStaticMeshComponent.GetInstanceTransform` _instancedstaticmesh_2 _index false)) (.rotation (`InstancedStaticMeshComponent.GetInstanceTransform` _instancedstaticmesh_2 _index false)) (`KismetMathLibrary.MakeVector` 0.5 0.5 (* (`|GetArrayItem` (`self.SpectrumValues`) _index) (`self.NodesSizeMultiplier`)))) false false true))
  ;[1 1 1] Apply all nodes new transform by setting same trasform to last element
  (`InstancedStaticMeshComponent.UpdateInstanceTransform` _instancedstaticmesh _returnvalue (`InstancedStaticMeshComponent.GetInstanceTransform` _instancedstaticmesh _returnvalue false) false true true))

(fn `SetIntensityToLight`
  (params (PointLight :type "PointLightComponent Object Reference") (SoundIntensity :type "Float (double-precision)") (DeltaTime :type "Float (double-precision)"))
  (`LightComponent.SetIntensity` PointLight (`KismetMathLibrary.FInterpTo` (`LightComponentBase.Intensity` PointLight) (+ (`KismetMathLibrary.FClamp` (* SoundIntensity (`self.LightIntensityMultiplier`)) 0.0 100000000.0) (`self.MinLightIntensity`)) DeltaTime (`self.LightInterpSpeed`))))

(fn `SetIntensityToLights`
  (params (SoundIntensity :type "Float (double-precision)") (DeltaTime :type "Float (double-precision)"))
  (for _array_element (`self.PointLights`)
    (`self.SetIntensityToLight` (`PointLight.PointLightComponent` _array_element) SoundIntensity DeltaTime)))

(fn `SetOnsetCubeScale`
  (params (RawIntensity :type "Float (double-precision)") (DeltaTime :type "Float (double-precision)"))
  (bind _strengthcube (`self.StrengthCube`))
  (`SceneComponent.SetRelativeScale3D` _strengthcube (`KismetMathLibrary.VLerp` (`SceneComponent.RelativeScale3D` _strengthcube) (`KismetMathLibrary.Conv_DoubleToVector` (* RawIntensity (`self.ActorSizeMultiplier`))) (* (`self.ActorInterpSpeed`) DeltaTime))))

(fn `SpawnEmitter`
  (`GameplayStatics.SpawnEmitterAtLocation` (`self.EmitterToSpawn`) (+ (`self.K2_GetActorLocation`) (0.0 0.0 500.0))))

(fn `SpawnNodes`
  (`StaticMeshComponent.SetStaticMesh` (`self.InstancedStaticMesh`) (`self.Node`))
  (`PrimitiveComponent.SetMaterial` (`self.InstancedStaticMesh`) 0 (`self.NodeMaterial`))
  (for _index (range (`self.Size`))
    (`InstancedStaticMeshComponent.AddInstance` (`self.InstancedStaticMesh`) (`KismetMathLibrary.MakeTransform` (`KismetMathLibrary.MakeVector` (.x (0.0 0.0 0.0)) (+ (.y (0.0 0.0 0.0)) (`KismetMathLibrary.Conv_IntToDouble` (* _index 100))) (.z (0.0 0.0 0.0)))))))

(fn `TickText`
  (bind _result (`self.FindTargetText`))
  (`/Game/Own/Blueprints/TextBP.SetText` (`self.SpawnedText`) _result))

(fn `UserConstructionScript`
  (bind _sound (`AudioAnalyzerNRT.Sound` (`self.LoudnessAnalizer`)))
  (`AudioComponent.SetSound` (`self.Audio`) _sound)
  (set `self.Duration` (`SoundBase.Duration` _sound)))