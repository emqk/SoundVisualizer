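; TextBP is a world-placed text label actor that displays text through a TextWidget component hosting a TextWidgetBP.
; On Tick, it rotates the whole actor to face LookAtActor whenever that reference is valid.
; SetText, SetColor and SetFontSize cast the hosted widget and update it, with text going through the widget's own SetText.
; SetFontSize rebuilds the font info, carrying over family, material, outline and typeface.
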(event `self.ReceiveTick`
  (params (DeltaSeconds :type "Float (single-precision)"))
  (bind _lookatactor (`self.LookAtActor`))
  (`/Engine/EditorBlueprintResources/StandardMacros.IsValid` _lookatactor
    (:`Is Valid`
      (`self.K2_SetActorRotation` (`KismetMathLibrary.FindLookAtRotation` (`self.K2_GetActorLocation`) (`self.K2_GetActorLocation` _lookatactor))))))

(fn `SetColor`
  (params (Color :type "SlateColor Structure"))
  (`TextBlock.SetColorAndOpacity` (`/Game/Own/Blueprints/TextWidgetBP.TextBlock_67` (cast `/Game/Own/Blueprints/TextWidgetBP` (`WidgetComponent.GetUserWidgetObject` (`self.TextWidget`)) :!pure true)) Color))

(fn `SetFontSize`
  (params (FontSize :type Integer))
  (bind _textblock_67 (`/Game/Own/Blueprints/TextWidgetBP.TextBlock_67` (cast `/Game/Own/Blueprints/TextWidgetBP` (`WidgetComponent.GetUserWidgetObject` (`self.TextWidget`)) :!pure true)))
  (bind (_fontobject _fontmaterial _outlinesettings _typefacefontname) (break `SlateFontInfo` (`TextBlock.Font` _textblock_67)))
  (`TextBlock.SetFont` _textblock_67 (make `SlateFontInfo` _fontobject _fontmaterial _outlinesettings _typefacefontname FontSize)))

(fn `SetText`
  (params (Text :type Text))
  (`/Game/Own/Blueprints/TextWidgetBP.SetText` (cast `/Game/Own/Blueprints/TextWidgetBP` (`WidgetComponent.GetUserWidgetObject` (`self.TextWidget`)) :!pure true) Text))

(fn `UserConstructionScript`)