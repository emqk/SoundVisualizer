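; Audio spectrum visualizer actor that shows spectrum values as bars built from instances of a single instanced static mesh.
; On BeginPlay it spawns the nodes in a line along Y or in a circle, depending on GenerationType.
; RefreshNodes takes an array of spectrum values and sets each instance's Z scale from them.
; It marks render state dirty only on a final re-set of the last instance, applying all updates at once.
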(event `self.ReceiveBeginPlay`
  (switch `/Game/Own/Blueprints/NodeVisType` (`self.GenerationType`)
    (:`NewEnumerator0`
      (`self.SpawnNodes`))
    (:`NewEnumerator1`
      (`self.SpawnNodesCircle`))))

(fn `RefreshNodes`
  (params (SpectrumValues :type "Array of Float (double-precision)"))
  (bind _instancedstaticmesh (`self.InstancedStaticMesh`))
  (bind _instancedstaticmesh_2 (`self.InstancedStaticMesh`))
  (bind _returnvalue (- (`KismetMathLibrary.Min` (`InstancedStaticMeshComponent.GetInstanceCount` _instancedstaticmesh_2) (`KismetArrayLibrary.Array_Length` SpectrumValues)) 1))
  ;[1 1 1] Refresh every node
  (for _index (range (+ _returnvalue 1))
    (`InstancedStaticMeshComponent.UpdateInstanceTransform` (`self.InstancedStaticMesh`) _index (`KismetMathLibrary.MakeTransform` (.location (`InstancedStaticMeshComponent.GetInstanceTransform` _instancedstaticmesh_2 _index false)) (.rotation (`InstancedStaticMeshComponent.GetInstanceTransform` _instancedstaticmesh_2 _index false)) (`KismetMathLibrary.MakeVector` 0.5 0.5 (* (`|GetArrayItem` SpectrumValues _index) (`self.NodeSizeMultiplier`)))) false false false))
  ;[1 1 1] Apply all nodes new transform by setting same trasform to last element
  (`InstancedStaticMeshComponent.UpdateInstanceTransform` _instancedstaticmesh _returnvalue (`InstancedStaticMeshComponent.GetInstanceTransform` _instancedstaticmesh _returnvalue false) false true false))

(fn `SpawnNodes`
  (`StaticMeshComponent.SetStaticMesh` (`self.InstancedStaticMesh`) (`self.NodeMesh`))
  (`PrimitiveComponent.SetMaterial` (`self.InstancedStaticMesh`) 0 (`self.NodeMaterial`))
  (for _index (range (`self.Size`))
    (`InstancedStaticMeshComponent.AddInstance` (`self.InstancedStaticMesh`) (`KismetMathLibrary.MakeTransform` (`KismetMathLibrary.MakeVector` (.x (0.0 0.0 0.0)) (+ (.y (0.0 0.0 0.0)) (* _index (* 100 (`self.NodeScaleMultiplier`)))) (.z (0.0 0.0 0.0))) (struct) (* (`KismetMathLibrary.MakeVector` 1.0 1.0 1.0) (`self.NodeScaleMultiplier`))))))

(fn `SpawnNodesCircle`
  (bind _size (`self.Size`))
  (`StaticMeshComponent.SetStaticMesh` (`self.InstancedStaticMesh`) (`self.NodeMesh`))
  (`PrimitiveComponent.SetMaterial` (`self.InstancedStaticMesh`) 0 (`self.NodeMaterial`))
  (for _index (range 1 (+ _size 1))
    (`InstancedStaticMeshComponent.AddInstance` (`self.InstancedStaticMesh`) (`KismetMathLibrary.MakeTransform` (+ (* (`KismetMathLibrary.GetForwardVector` (`KismetMathLibrary.MakeRotator` 0.0 0.0 (* _index (/ 360.0 (`KismetMathLibrary.Conv_IntToDouble` _size))))) (`self.CircleRadius`)) (`self.K2_GetActorLocation`))))))

(fn `UserConstructionScript`)