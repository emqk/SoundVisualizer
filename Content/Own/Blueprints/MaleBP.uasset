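; MaleBP is a male character Blueprint whose eye material blends smoothly toward a requested color amount.
; The construction script creates a dynamic material instance on the Eyes component.
; SetDynamicMaterialColorAmount stores a target value, and Tick eases the material's LerpAmount parameter toward it with FInterpTo at LerpSpeed.
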(event `self.ReceiveTick`
  (params (DeltaSeconds :type "Float (single-precision)"))
  (bind _returnvalue (`MaterialInstanceDynamic.K2_GetScalarParameterValue` (`self.EyesDynamicMat`) "LerpAmount"))
  (`MaterialInstanceDynamic.SetScalarParameterValue` (`self.EyesDynamicMat`) "LerpAmount" (`KismetMathLibrary.FInterpTo` _returnvalue (`self.ColorAmount`) DeltaSeconds (`self.LerpSpeed`))))

(fn `SetDynamicMaterialColorAmount`
  (params (Amount01 :type "Float (double-precision)"))
  (set `self.ColorAmount` Amount01))

(fn `UserConstructionScript`
  (bind _returnvalue (`PrimitiveComponent.CreateDynamicMaterialInstance` (`self.Eyes`) 0 null "None"))
  (set `self.EyesDynamicMat` _returnvalue))